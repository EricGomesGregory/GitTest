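; BP_CharacterInteraction handles player interaction with world objects through a camera-based line trace.
; InteractAction traces on the Visibility channel between the origin and direction returned by GetRayDirection.
; If the hit actor implements BPI_Interactable and CanInteract is true, it receives OnInteractedMessage.
; GetRayDirection's only logic, camera location plus forward vector times Range, is left unused.
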(fn InteractAction
  (params (camera :type Camera%20Component%20Object%20Reference))
  (bind _range (Variables|Default|GetRange))
  (bind (_origin _direction) (Utilities|GetRayDirection camera _range))
  (bind _outhit (Collision|LineTraceByChannel _origin _direction "TraceTypeQuery1" false 0 "None"))
  (if (Utilities|DoesObjectImplementInterface (.HitActor (Collision|BreakHitResult _outhit)) "/Game/Blueprints/Interactables/BPI_Interactable.BPI_Interactable_C")
    (if (Variables|Default|GetCan%20Interact)
      (Class|BPIInteractable|OnInteracted(Message) (.HitActor (Collision|BreakHitResult _outhit))))))